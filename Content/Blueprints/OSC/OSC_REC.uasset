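; OSC receiver Blueprint that triggers Level Sequence playback from incoming network OSC messages.
; On BeginPlay it creates and stores a listening OSC server on port 8000 across all interfaces, then binds a message-received handler.
; The receive event plays the referenced sequence without filtering by address; the address path and debug print nodes are left disconnected.
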(event `self.ReceiveBeginPlay`
  (bind _returnvalue (`OSCManager.CreateOSCServer` "0.0.0.0" 8000 false true "" null))
  (bind _output_get (set `self.OSCSever` _returnvalue))
  (clear `OSCServer.OnOscBundleReceived` _output_get)
  (add `OSCServer.OnOscMessageReceived` _output_get (`|CreateDelegate` :!event `OSCRecieve`)))

(event `OSCRecieve`
  (params (Message :type "OSCMessage Structure (by ref)") (IPAddress :type String) (Port :type Integer))
  (bind _returnvalue (`OSCManager.GetOSCMessageAddress` Message))
  (`MovieSceneSequencePlayer.Play` (`LevelSequenceActor.SequencePlayer` (`self.LevelSequence`))))

(fn `UserConstructionScript`)